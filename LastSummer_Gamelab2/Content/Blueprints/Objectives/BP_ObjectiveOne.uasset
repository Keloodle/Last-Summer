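; Placeable objective actor that gives the player a task of collecting items, building a treehouse or walking to a spot.
; Player overlap with ObjectiveEnd activates the task in its own WBP_Objectives widget, while ObjectiveStart overlaps drive completion.
; Collection counts matching BP_ItemParent actors in the volume, and the treehouse type adds a camera fade and mesh swap.
; Completing an active task notifies BP_ObjectiveManager and updates the widget.
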(event `self.ObjectiveEnd.OnComponentBeginOverlap`
  (params (OverlappedComponent :type "PrimitiveComponent Object Reference") (OtherActor :type "Actor Object Reference") (OtherComp :type "PrimitiveComponent Object Reference") (OtherBodyIndex :type Integer) (bFromSweep :type Boolean) (SweepResult :type "HitResult Structure (by ref)"))
  (cast `/Game/FirstPerson/Blueprints/BP_FirstPersonCharacter` OtherActor)
  (`self.UpdateObjective` (`self.SetNewObjective`)))

(event `self.ReceiveBeginPlay`
  (`self.StartObjective`))

(event `self.ReceiveTick`
  (params (DeltaSeconds :type "Float (single-precision)")))

(event `self.ObjectiveStart.OnComponentBeginOverlap`
  (params (OverlappedComponent :type "PrimitiveComponent Object Reference") (OtherActor :type "Actor Object Reference") (OtherComp :type "PrimitiveComponent Object Reference") (OtherBodyIndex :type Integer) (bFromSweep :type Boolean) (SweepResult :type "HitResult Structure (by ref)"))
  (switch `/Game/Blueprints/Objectives/Enum_ObjectiveTypes` (`self.ObjectieType`)
    (:`NewEnumerator0`
      (`self.CollectionTask` OtherActor))
    (:`NewEnumerator1`
      (`self.CollectionTask` OtherActor)
      (`self.fadeToBlackEvent`))
    (:`NewEnumerator3`
      _))
  (`self.Complete` (`self.ObjectiveTask`)))

(event `self.ObjectiveStart.OnComponentEndOverlap`
  (params (OverlappedComponent :type "PrimitiveComponent Object Reference") (OtherActor :type "Actor Object Reference") (OtherComp :type "PrimitiveComponent Object Reference") (OtherBodyIndex :type Integer))
  (`self.CollectionFailTask` OtherActor))

(fn `CollectionFailTask`
  (params (Actor :type "Actor Object Reference"))
  (bind _asbp_item_parent (cast `/Game/Blueprints/Pickups/BP_ItemParent` Actor))
  (if (`KismetTextLibrary.EqualEqual_TextText` (`/Game/Blueprints/Pickups/BP_ItemParent.ItemType` _asbp_item_parent) (`self.ItemType`))
    (bind _result (`/Engine/EditorBlueprintResources/StandardMacros.DecrementInt` (`self.Inventory`))
      (:`  `
        (`KismetSystemLibrary.PrintString` (`KismetStringLibrary.Conv_IntToString` _result))
        (return)))))

(fn `CollectionTask`
  (params (Actor :type "Actor Object Reference"))
  (if (not (`self.IsChatObjecive`))
    (bind _asbp_item_parent (cast `/Game/Blueprints/Pickups/BP_ItemParent` Actor))
    (if (`KismetTextLibrary.EqualEqual_TextText` (`/Game/Blueprints/Pickups/BP_ItemParent.ItemType` _asbp_item_parent) (`self.ItemType`))
      (bind _result (`/Engine/EditorBlueprintResources/StandardMacros.IncrementInt` (`self.Inventory`))
        (:`  `
          (`KismetSystemLibrary.PrintString` (`KismetStringLibrary.Conv_IntToString` _result))
          (if (== (`self.Inventory`) (`self.MaxTargets`))
            (return)))))))

(fn `Complete`
  (params (ObjectiveToComplete :type "/Game/Blueprints/Objectives/Enum_Objectives Enum" :default "NewEnumerator0"))
  (switch `/Game/Blueprints/Objectives/Enum_Objectives` ObjectiveToComplete
    (:`NewEnumerator0`
      (if (`self.ObjOneActive`)
        (bind _returnvalue (`GameplayStatics.GetActorOfClass` "/Game/Blueprints/Objectives/BP_ObjectiveManager.BP_ObjectiveManager_C"))
        (`self.ObjectiveCompleted` _returnvalue)
        (`/Game/Blueprints/UI/WBP_Objectives.CheckObjectives` (`self.ObjectiveWidget`) ObjectiveToComplete :!label _label)))
    (:`NewEnumerator1`
      (if (`self.ObjTwoActive`)
        (bind _returnvalue_2 (`GameplayStatics.GetActorOfClass` "/Game/Blueprints/Objectives/BP_ObjectiveManager.BP_ObjectiveManager_C"))
        (`self.ObjectiveCompleted` _returnvalue_2)
        (goto _label)))
    (:`NewEnumerator2`
      (if (`self.ObjThreeActive`)
        (bind _returnvalue_3 (`GameplayStatics.GetActorOfClass` "/Game/Blueprints/Objectives/BP_ObjectiveManager.BP_ObjectiveManager_C"))
        (`self.ObjectiveCompleted` _returnvalue_3)
        (goto _label)))
    (:`NewEnumerator3`
      (if (`self.ObjFourActive`)
        (bind _returnvalue_4 (`GameplayStatics.GetActorOfClass` "/Game/Blueprints/Objectives/BP_ObjectiveManager.BP_ObjectiveManager_C"))
        (`self.ObjectiveCompleted` _returnvalue_4)
        (goto _label)))
    (:`NewEnumerator5`
      (if (`self.ObjMainActive`)
        (bind _returnvalue_5 (`GameplayStatics.GetActorOfClass` "/Game/Blueprints/Objectives/BP_ObjectiveManager.BP_ObjectiveManager_C"))
        (`self.MainObjective` _returnvalue_5)
        (goto _label)))))

(fn `fadeToBlackEvent`
  (bind _returnvalue (`GameplayStatics.GetPlayerCameraManager` 0))
  (`PlayerCameraManager.StartCameraFade` :`self` _returnvalue :`ToAlpha` 4.0 :`Duration` 2.0)
  (`StaticMeshComponent.SetStaticMesh` (`self.EmptyMesh`) (`self.MeshToSpawn`))
  (`PlayerCameraManager.StartCameraFade` :`self` _returnvalue :`FromAlpha` 4.0 :`Duration` 2.0))

(fn `OpenDoor`
  (params (Interactor :type "Character Object Reference"))
  (returns (`Did Interact` :type Boolean))
  (return false))

(fn `StartObjective`
  (bind _returnvalue (`|CreateWidget` "/Game/Blueprints/UI/WBP_Objectives.WBP_Objectives_C" (`GameplayStatics.GetPlayerController` 0)))
  (bind _output_get (set `self.ObjectiveWidget` _returnvalue))
  (`UserWidget.AddToViewport` _output_get 0)
  (`KismetSystemLibrary.PrintString` "create widget"))

(fn `UpdateObjective`
  (params (`New Objective` :type Text))
  (bind _objectivetask (`self.ObjectiveTask`))
  (`/Game/Blueprints/UI/WBP_Objectives.AddObjective` (`self.ObjectiveWidget`) _objectivetask `New Objective`)
  (switch `/Game/Blueprints/Objectives/Enum_Objectives` _objectivetask
    (:`NewEnumerator0`
      (set `self.ObjOneActive` true)
      (`KismetSystemLibrary.PrintString` "one"))
    (:`NewEnumerator1`
      (set `self.ObjTwoActive` true)
      (`KismetSystemLibrary.PrintString` "two"))
    (:`NewEnumerator2`
      (set `self.ObjThreeActive` true)
      (`KismetSystemLibrary.PrintString` "thre"))
    (:`NewEnumerator3`
      (set `self.ObjFourActive` true)
      (`KismetSystemLibrary.PrintString` "four"))
    (:`NewEnumerator5`
      (set `self.ObjMainActive` true)
      (`KismetSystemLibrary.PrintString` "main"))))

(fn `UserConstructionScript`)