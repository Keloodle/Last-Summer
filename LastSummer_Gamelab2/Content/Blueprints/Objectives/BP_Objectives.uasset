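; BP_Objectives is a trigger actor that shows objective text on screen when the player reaches it.
; The first overlap of its Trigger by BP_FirstPersonCharacter fires Update, which writes the stored Objective to the ObjectiveWidget text and ignores its parameter.
; A separate UpdateObjective function stores a new objective and refreshes the same text.
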(event `self.Trigger.OnComponentBeginOverlap`
  (params (OverlappedComponent :type "PrimitiveComponent Object Reference") (OtherActor :type "Actor Object Reference") (OtherComp :type "PrimitiveComponent Object Reference") (OtherBodyIndex :type Integer) (bFromSweep :type Boolean) (SweepResult :type "HitResult Structure (by ref)"))
  (cast `/Game/FirstPerson/Blueprints/BP_FirstPersonCharacter` OtherActor)
  (`/Engine/EditorBlueprintResources/StandardMacros.DoOnce` false
    (:`Completed`
      (`self.Update` ""))))

(event `Update`
  (params (NewParam :type String))
  (`TextBlock.SetText` (`/Game/Blueprints/UI/WBP_Objectives.Objectivetext` (`self.ObjectiveWidget`)) (`KismetTextLibrary.Conv_StringToText` (`self.Objective`))))

(fn `UpdateObjective`
  (params (`Current Objective` :type String))
  (set `self.Objective` `Current Objective`)
  (`TextBlock.SetText` (`/Game/Blueprints/UI/WBP_Objectives.Objectivetext` (`self.ObjectiveWidget`)) (`KismetTextLibrary.Conv_StringToText` (`self.Objective`))))

(fn `UserConstructionScript`)