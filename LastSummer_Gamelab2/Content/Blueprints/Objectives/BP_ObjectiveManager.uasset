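; BP_ObjectiveManager tracks one main and four side objectives and loads Level1 once they are done.
; BeginPlay creates the objectives and loading screen widgets and shows the cursor.
; Interface events activate objectives and, for active ones only, update the widget and either increment the side count or flag the main as complete.
; Tick waits for the count to exceed its threshold with main complete, then fades the loading screen and opens the level.
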(event `self.ReceiveBeginPlay`
  (bind _returnvalue (`GameplayStatics.GetPlayerController` 0))
  (bind _returnvalue_2 (`|CreateWidget` "/Game/Blueprints/UI/WBP_Objectives.WBP_Objectives_C" _returnvalue))
  (set `PlayerController.bShowMouseCursor` true _returnvalue)
  (bind _output_get (set `self.ObjectiveWidget` _returnvalue_2))
  (`UserWidget.AddToViewport` _output_get 0)
  (`KismetSystemLibrary.PrintString` "create widget manger")
  (bind _returnvalue_3 (`|CreateWidget` "/Game/Blueprints/UI/WBP_LoadingScreen.WBP_LoadingScreen_C"))
  (bind _output_get_2 (set `self.LoadingScreen` _returnvalue_3))
  (`UserWidget.AddToViewport` _output_get_2 0)
  (`UserWidget.PlayAnimation` _output_get_2 (`/Game/Blueprints/UI/WBP_LoadingScreen.FadeIn` _output_get_2) 0.0 1 "Forward" 1.0 false))

(event `/Game/Blueprints/Pickups/Interact_Interface.UpdateObjectiveInterface`
  (params (`New Objective` :type Text) (ObjectiveTask :type "/Game/Blueprints/Objectives/Enum_Objectives Enum" :default "NewEnumerator0"))
  (`/Game/Blueprints/UI/WBP_Objectives.AddObjective` (`self.ObjectiveWidget`) ObjectiveTask `New Objective`)
  (switch `/Game/Blueprints/Objectives/Enum_Objectives` ObjectiveTask
    (:`NewEnumerator0`
      (set `self.ObjOneActive` true)
      (`KismetSystemLibrary.PrintString` "one"))
    (:`NewEnumerator1`
      (set `self.ObjTwoActive` true)
      (`KismetSystemLibrary.PrintString` "two"))
    (:`NewEnumerator2`
      (set `self.ObjThreeActive` true)
      (`KismetSystemLibrary.PrintString` "thre"))
    (:`NewEnumerator3`
      (set `self.ObjFourActive` true)
      (`KismetSystemLibrary.PrintString` "four"))
    (:`NewEnumerator5`
      (set `self.ObjMainActive` true)
      (`KismetSystemLibrary.PrintString` "main"))))

(event `self.ReceiveTick`
  (params (DeltaSeconds :type "Float (single-precision)"))
  (if (and (> (`self.SideObjectiveCount`) (`self.SideObjectiveToComplete`)) (`self.ObjMainComplete`))
    (`/Engine/EditorBlueprintResources/StandardMacros.DoOnce` false
      (:`Completed`
        (`/Game/Blueprints/UI/WBP_LoadingScreen.FadeInAnimation` (`self.Loadingscreen`))
        (`KismetSystemLibrary.Delay` 2.0)
        (`GameplayStatics.OpenLevel` "Level1")))))

(event `/Game/Blueprints/Pickups/Interact_Interface.ObjectivesCompletedCount`
  (bind _result (`/Engine/EditorBlueprintResources/StandardMacros.IncrementInt` (`self.SideObjectiveCount`))
    (:`  `
      (`KismetSystemLibrary.PrintString` (`KismetStringLibrary.Conv_IntToString` _result)))))

(event `/Game/Blueprints/Pickups/Interact_Interface.MainObjective`
  (bind _output_get (set `self.ObjMainComplete` true))
  (`KismetSystemLibrary.PrintString` (`KismetStringLibrary.Conv_BoolToString` _output_get)))

(event `/Game/Blueprints/Pickups/Interact_Interface.CompleteObjectiveInterface`
  (params (ObjectiveToComplete :type "/Game/Blueprints/Objectives/Enum_Objectives Enum" :default "NewEnumerator0"))
  (switch `/Game/Blueprints/Objectives/Enum_Objectives` ObjectiveToComplete
    (:`NewEnumerator0`
      (if (`self.ObjOneActive`)
        (bind _returnvalue (`GameplayStatics.GetActorOfClass` "BP_ObjectiveManager_C"))
        (`/Game/Blueprints/Pickups/Interact_Interface.ObjectivesCompletedCount` _returnvalue)
        (`/Game/Blueprints/UI/WBP_Objectives.CheckObjectives` (`self.ObjectiveWidget`) ObjectiveToComplete :!label _label)))
    (:`NewEnumerator1`
      (if (`self.ObjTwoActive`)
        (bind _returnvalue_2 (`GameplayStatics.GetActorOfClass` "BP_ObjectiveManager_C"))
        (`/Game/Blueprints/Pickups/Interact_Interface.ObjectivesCompletedCount` _returnvalue_2)
        (goto _label)))
    (:`NewEnumerator2`
      (if (`self.ObjThreeActive`)
        (bind _returnvalue_3 (`GameplayStatics.GetActorOfClass` "BP_ObjectiveManager_C"))
        (`/Game/Blueprints/Pickups/Interact_Interface.ObjectivesCompletedCount` _returnvalue_3)
        (goto _label)))
    (:`NewEnumerator3`
      (if (`self.ObjFourActive`)
        (bind _returnvalue_4 (`GameplayStatics.GetActorOfClass` "BP_ObjectiveManager_C"))
        (`/Game/Blueprints/Pickups/Interact_Interface.ObjectivesCompletedCount` _returnvalue_4)
        (goto _label)))
    (:`NewEnumerator5`
      (if (`self.ObjMainActive`)
        (bind _returnvalue_5 (`GameplayStatics.GetActorOfClass` "BP_ObjectiveManager_C"))
        (`/Game/Blueprints/Pickups/Interact_Interface.MainObjective` _returnvalue_5)
        (goto _label)))))

(fn `OpenDoor`
  (params (Interactor :type "Character Object Reference"))
  (returns (`Did Interact` :type Boolean))
  (return false))

(fn `UserConstructionScript`)