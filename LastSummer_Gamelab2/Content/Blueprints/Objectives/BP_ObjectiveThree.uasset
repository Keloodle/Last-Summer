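; BP_ObjectiveThree is an objective trigger actor that posts the third objective to the player's on-screen objectives UI.
; When BP_FirstPersonCharacter first overlaps its Trigger, a DoOnce creates and displays a WBP_Objectives widget if its ObjectiveWidget reference is invalid.
; It then passes SetNewObjective through UpdateObjective to the widget's AddObjectiveThree.
; A generic AddObjective call is left unconnected.
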(event `self.ReceiveBeginPlay`)

(event `self.Trigger.OnComponentBeginOverlap`
  (params (OverlappedComponent :type "PrimitiveComponent Object Reference") (OtherActor :type "Actor Object Reference") (OtherComp :type "PrimitiveComponent Object Reference") (OtherBodyIndex :type Integer) (bFromSweep :type Boolean) (SweepResult :type "HitResult Structure (by ref)"))
  (cast `/Game/FirstPerson/Blueprints/BP_FirstPersonCharacter` OtherActor)
  (`/Engine/EditorBlueprintResources/StandardMacros.DoOnce` false
    (:`Completed`
      (`self.ObjectiveWidget`
        (:`then`
          _)
        (:`else`
          (`self.StartObjective`)))
      (`self.UpdateObjective` (`self.SetNewObjective`)))))

(fn `StartObjective`
  (bind _returnvalue (`|CreateWidget` "/Game/Blueprints/UI/WBP_Objectives.WBP_Objectives_C" (`GameplayStatics.GetPlayerController` 0)))
  (bind _output_get (set `self.ObjectiveWidget` _returnvalue))
  (`UserWidget.AddToViewport` _output_get 0))

(fn `UpdateObjective`
  (params (`New Objective` :type Text))
  (`/Game/Blueprints/UI/WBP_Objectives.AddObjectiveThree` (`self.ObjectiveWidget`) `New Objective`))

(fn `UserConstructionScript`)