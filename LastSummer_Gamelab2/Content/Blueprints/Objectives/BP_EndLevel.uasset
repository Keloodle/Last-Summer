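; Level exit objective that lets the first-person character end the game from inside the End overlap volume.
; CanPlayerEnd unlocks it, after which entering the volume sets CanInteract and leaving clears it.
; When CanInteract is set, TheEnd shows WBP_TheEnd, pauses the game, disables its own input, shows the cursor and plays the ending fade.
; OpenDoor is a stub that returns false.
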(event `/Game/Blueprints/Pickups/Interact_Interface.TheEnd`
  (bind _returnvalue (`GameplayStatics.GetPlayerController` 0))
  (if (`self.CanInteract`)
    (bind _returnvalue_2 (`|CreateWidget` "/Game/Blueprints/UI/WBP_TheEnd.WBP_TheEnd_C" _returnvalue))
    (bind _output_get (set `self.NewVar` _returnvalue_2))
    (`UserWidget.AddToViewport` _output_get 0)
    (`GameplayStatics.SetGamePaused` true)
    (`self.DisableInput` _returnvalue)
    (set `PlayerController.bShowMouseCursor` true _returnvalue)
    (`UserWidget.PlayAnimation` _output_get (`/Game/Blueprints/UI/WBP_TheEnd.FadeEnding` _output_get) 0.0 1 "Forward" 1.0 false)))

(event `/Game/Blueprints/Pickups/Interact_Interface.CanPlayerEnd`
  (set `self.CanEnd` true))

(event `self.End.OnComponentBeginOverlap`
  (params (OverlappedComponent :type "PrimitiveComponent Object Reference") (OtherActor :type "Actor Object Reference") (OtherComp :type "PrimitiveComponent Object Reference") (OtherBodyIndex :type Integer) (bFromSweep :type Boolean) (SweepResult :type "HitResult Structure (by ref)"))
  (cast `/Game/FirstPerson/Blueprints/BP_FirstPersonCharacter` OtherActor)
  (if (`self.CanEnd`)
    (set `self.CanInteract` true)))

(event `self.End.OnComponentEndOverlap`
  (params (OverlappedComponent :type "PrimitiveComponent Object Reference") (OtherActor :type "Actor Object Reference") (OtherComp :type "PrimitiveComponent Object Reference") (OtherBodyIndex :type Integer))
  (cast `/Game/FirstPerson/Blueprints/BP_FirstPersonCharacter` OtherActor)
  (set `self.CanInteract` false))

(fn `OpenDoor`
  (params (Interactor :type "Character Object Reference"))
  (returns (`Did Interact` :type Boolean))
  (return false))

(fn `UserConstructionScript`)