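; BP_ObjectiveField is a trigger zone that counts objective items placed inside its box.
; Box overlap events cast the other actor to BP_ItemParent and compare its ItemType to ObjectiveTarget, raising Inventory on entry and lowering it on exit.
; Each change prints the count, and reaching MaxTargets on entry only prints a placeholder "Hello", with no completion logic yet.
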(event `self.Box.OnComponentBeginOverlap`
  (params (OverlappedComponent :type "PrimitiveComponent Object Reference") (OtherActor :type "Actor Object Reference") (OtherComp :type "PrimitiveComponent Object Reference") (OtherBodyIndex :type Integer) (bFromSweep :type Boolean) (SweepResult :type "HitResult Structure (by ref)"))
  (bind _asbp_item_parent (cast `/Game/Blueprints/Pickups/BP_ItemParent` OtherActor))
  (if (`KismetTextLibrary.EqualEqual_TextText` (`/Game/Blueprints/Pickups/BP_ItemParent.ItemType` _asbp_item_parent) (`self.ObjectiveTarget`))
    (bind _result (`/Engine/EditorBlueprintResources/StandardMacros.IncrementInt` (`self.Inventory`))
      (:`  `
        (`KismetSystemLibrary.PrintString` (`KismetStringLibrary.Conv_IntToString` _result))
        (if (== (`self.Inventory`) (`self.MaxTargets`))
          (`KismetSystemLibrary.PrintString` "Hello"))))))

(event `self.Box.OnComponentEndOverlap`
  (params (OverlappedComponent :type "PrimitiveComponent Object Reference") (OtherActor :type "Actor Object Reference") (OtherComp :type "PrimitiveComponent Object Reference") (OtherBodyIndex :type Integer))
  (bind _asbp_item_parent (cast `/Game/Blueprints/Pickups/BP_ItemParent` OtherActor))
  (if (`KismetTextLibrary.EqualEqual_TextText` (`/Game/Blueprints/Pickups/BP_ItemParent.ItemType` _asbp_item_parent) (`self.ObjectiveTarget`))
    (bind _result (`/Engine/EditorBlueprintResources/StandardMacros.DecrementInt` (`self.Inventory`))
      (:`  `
        (`KismetSystemLibrary.PrintString` (`KismetStringLibrary.Conv_IntToString` _result))))))

(fn `UserConstructionScript`)