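; BP_CompleteObjective is a trigger actor that completes an objective when the first-person player character enters its box.
; The box overlap filters for BP_FirstPersonCharacter, prints a debug string, then calls CompleteObjective, which passes ObjectiveToCheck to the Complete function on Objective.
; Disconnected leftover nodes for tinting an objective widget green and printing a message never run.
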(event `self.ReceiveBeginPlay`)

(event `self.Box.OnComponentBeginOverlap`
  (params (OverlappedComponent :type "PrimitiveComponent Object Reference") (OtherActor :type "Actor Object Reference") (OtherComp :type "PrimitiveComponent Object Reference") (OtherBodyIndex :type Integer) (bFromSweep :type Boolean) (SweepResult :type "HitResult Structure (by ref)"))
  (cast `/Game/FirstPerson/Blueprints/BP_FirstPersonCharacter` OtherActor)
  (`KismetSystemLibrary.PrintString` "trigger")
  (`self.CompleteObjective`))

(fn `CompleteObjective`
  (`/Game/Blueprints/Objectives/BP_ObjectiveOne.Complete` (`self.Objective`) (`self.ObjectiveToCheck`)))

(fn `UserConstructionScript`)