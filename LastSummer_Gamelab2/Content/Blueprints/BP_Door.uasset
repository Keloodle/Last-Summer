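; BP_Door is an interactable door that swings open and closed when OpenDoor is called while the first-person character is inside its Box trigger.
; Box overlaps set CanInteract, which Tick uses to show or hide the press prompt in a WBP_DoorInterface widget created on BeginPlay.
; One timeline lerps the mesh's yaw, playing or reversing at rates derived from TimeToOpen and TimeToClose, and flips IsOpen when finished.
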(event `self.ReceiveBeginPlay`
  (bind _returnvalue (`|CreateWidget` "/Game/Blueprints/UI/WBP_DoorInterface.WBP_DoorInterface_C"))
  (bind _output_get (set `self.DoorInterface` _returnvalue))
  (`UserWidget.AddToViewport` _output_get 0))

(event `self.ReceiveTick`
  (params (DeltaSeconds :type "Float (single-precision)"))
  (bind _pressborder (`/Game/Blueprints/UI/WBP_DoorInterface.PressBorder` (`self.DoorInterface`)))
  (if (`self.CanInteract`)
    (`Widget.SetVisibility` _pressborder "Visible")
    (else
      (`Widget.SetVisibility` _pressborder "Hidden"))))

(event `Open`
  (bind (_direction _doortrack) (`Timeline|OpenDoorT` :!label _label)
    (:`Update`
      (`SceneComponent.K2_SetRelativeRotation` (`self.Door SM`) (`KismetMathLibrary.MakeRotator` 0.0 0.0 (`KismetMathLibrary.Lerp` (`self.ClosePosition`) (`self.OpenPosition`) _doortrack)) false false))
    (:`Finished`
      (set `self.IsOpen` (not (`self.IsOpen`))))))

(event `Close`
  (goto _label :!via `Reverse`))

(event `self.Box.OnComponentBeginOverlap`
  (params (OverlappedComponent :type "PrimitiveComponent Object Reference") (OtherActor :type "Actor Object Reference") (OtherComp :type "PrimitiveComponent Object Reference") (OtherBodyIndex :type Integer) (bFromSweep :type Boolean) (SweepResult :type "HitResult Structure (by ref)"))
  (cast `/Game/FirstPerson/Blueprints/BP_FirstPersonCharacter` OtherActor)
  (set `self.CanInteract` true))

(event `self.Box.OnComponentEndOverlap`
  (params (OverlappedComponent :type "PrimitiveComponent Object Reference") (OtherActor :type "Actor Object Reference") (OtherComp :type "PrimitiveComponent Object Reference") (OtherBodyIndex :type Integer))
  (cast `/Game/FirstPerson/Blueprints/BP_FirstPersonCharacter` OtherActor)
  (set `self.CanInteract` false))

(fn `OpenDoor`
  (params (Interactor :type "Character Object Reference"))
  (returns (`Did Interact` :type Boolean))
  (bind _opendoort (`self.OpenDoorT`))
  (if (`self.CanInteract`)
    (if (not (`self.IsOpen`))
      (`TimelineComponent.SetPlayRate` _opendoort (/ 1.0 (`self.TimeToOpen`)))
      (`self.Open`)
      (else
        (`TimelineComponent.SetPlayRate` _opendoort (/ 1.0 (`self.TimeToClose`)))
        (`self.Close`)))
    (return false)))

(fn `UserConstructionScript`)